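; BP_Building is a building actor that drives a PCG graph to lay out modular floors and walls.
; Its construction script derives floor offset and scale, per-direction wall offsets and a wall-centering offset from the wall and floor sizes.
; It also computes a height offset from wall height and floor count for multiple storeys.
; All values are pushed as vector parameters to the PCG graph instance, with no runtime logic.
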(event EventBeginPlay)

(event Collision|EventActorBeginOverlap
  (params (OtherActor :type Actor%20Object%20Reference)))

(event EventTick
  (params (DeltaSeconds :type Float%20%28single-precision%29)))

(fn ConstructionScript
  (bind _pcg (Variables|Default|GetPCG))
  (bind _wallsize (Variables|Default|GetWallSize))
  (bind _wallsize_2 (Variables|Default|GetWallSize))
  (bind _returnvalue (/ _wallsize 2.0))
  (bind _returnvalue_2 (/ _wallsize_2 2.0))
  (bind _graphinstance (Variables|/Script/PCG.PCGComponent|GetGraphInstance _pcg))
  (bind _returnvalue_3 (* _returnvalue -1.0))
  (bind _returnvalue_4 (* _returnvalue_2 -1.0))
  ;[1 1 1] Floor Params
  (Effects|Components|ParticleSystem|SetVectorParameter _graphinstance "FloorOffset" (Math|Vector|MakeVector _returnvalue_3 _returnvalue_3 0.0))
  (Effects|Components|ParticleSystem|SetVectorParameter _graphinstance "FloorScale" (Math|Conversions|ToVector(Float) (/ (Variables|Default|GetWallSize) (Variables|Default|GetFloorSize))))
  ;[1 1 1] Wall Params
  (Effects|Components|ParticleSystem|SetVectorParameter _graphinstance "WallOffsetN" (Math|Vector|MakeVector _returnvalue_2 0.0 0.0))
  (Effects|Components|ParticleSystem|SetVectorParameter _graphinstance "WallOffsetE" (Math|Vector|MakeVector 0.0 _returnvalue_2 0.0))
  (Effects|Components|ParticleSystem|SetVectorParameter _graphinstance "WallOffsetS" (Math|Vector|MakeVector _returnvalue_4 0.0 0.0))
  (Effects|Components|ParticleSystem|SetVectorParameter _graphinstance "WallOffsetW" (Math|Vector|MakeVector 0.0 _returnvalue_4 0.0))
  ;[1 1 1] Centering Walls on Points
  (Effects|Components|ParticleSystem|SetVectorParameter _graphinstance "UnivWallOffset" (Math|Vector|MakeVector 0.0 (* (/ (Variables|Default|GetWallSize) 2.0) -1.0) 0.0))
  ;[1 1 1] Multiple Floors
  (Effects|Components|ParticleSystem|SetVectorParameter _graphinstance "FloorHeightOffset" (Math|Vector|MakeVector 0.0 0.0 (* (Variables|Default|GetWallHeight) (- (Variables|Default|GetNumFloors) 1)))))